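; BP_Sword is a melee weapon Blueprint that extends a parent weapon class with a capsule hitbox for dealing sword damage.
; The capsule's collision starts disabled and is toggled by the OnCollision and OffCollision events, regardless of the fist collision type passed in.
; Each overlap sends the single damage value from WeaponDamageComponent to the other actor.
; Combo start and end events also start and end that component's attack.
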(event `self.ReceiveBeginPlay`
  (`parent.ReceiveBeginPlay`)
  (`PrimitiveComponent.SetCollisionEnabled` (`self.Capsule`) "NoCollision"))

(event `self.Capsule.OnComponentBeginOverlap`
  (params (OverlappedComponent :type "PrimitiveComponent Object Reference") (OtherActor :type "Actor Object Reference") (OtherComp :type "PrimitiveComponent Object Reference") (OtherBodyIndex :type Integer) (bFromSweep :type Boolean) (SweepResult :type "HitResult Structure (by ref)"))
  (bind _attack (`/Game/Components/WeaponDamageComponent.GetSingleDamage` (`self.WeaponDamageComponent`)))
  (`self.SendDamage` OtherActor _attack))

(event `self.StartCombo`
  (`parent.StartCombo`)
  (`/Game/Components/WeaponDamageComponent.StartAttack` (`self.WeaponDamageComponent`)))

(event `self.EndCombo`
  (`parent.EndCombo`)
  (`/Game/Components/WeaponDamageComponent.EndAttack` (`self.WeaponDamageComponent`)))

(event `self.OnCollision`
  (params (FistCollisionType :type "/Game/Enums/EFistCollisionType Enum" :default "NewEnumerator0"))
  (`parent.OnCollision` FistCollisionType)
  (`PrimitiveComponent.SetCollisionEnabled` (`self.Capsule`) "QueryAndPhysics"))

(event `self.OffCollision`
  (`parent.OffCollision`)
  (`PrimitiveComponent.SetCollisionEnabled` (`self.Capsule`) "NoCollision"))

(fn `UserConstructionScript`)