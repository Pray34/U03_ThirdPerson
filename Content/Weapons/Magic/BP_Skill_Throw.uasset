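; BP_Skill_Throw is a magic skill weapon that lets the player throw one of several configured items.
; Equipping shows the current item's attached particle and turns on player aim; unequipping reverses both.
; Spell plays a fireball montage, while a separate Throw event spawns the item from the Hand_Throw socket along the control rotation.
; SetCurrentItem selects the ThrowItems entry by class and swaps the particle template.
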(event `self.ReceiveBeginPlay`
  (bind (_output_throwitemclass _output_attachparticle) (break `/Game/Structs/FThrowItem` (`|GetArrayItem` (`self.ThrowItems`) (`self.CurrentItem`))))
  (`ParticleSystemComponent.SetTemplate` (`self.AttachParticle`) _output_attachparticle)
  (`SceneComponent.SetVisibility` (`self.AttachParticle`) false false))

(event `self.OnEquipped`
  (`parent.OnEquipped`)
  (`SceneComponent.SetVisibility` (`self.AttachParticle`) true false)
  (bind _asbp_player (cast `/Game/Player/BP_Player` (`self.GetOwnerToCharacter`)))
  (`/Game/Player/BP_Player.OnAim` _asbp_player))

(event `self.OnUnequipped`
  (`parent.OnUnequipped`)
  (`SceneComponent.SetVisibility` (`self.AttachParticle`) false false)
  (bind _asbp_player (cast `/Game/Player/BP_Player` (`self.GetOwnerToCharacter`)))
  (`/Game/Player/BP_Player.OffAim` _asbp_player))

(event `self.Spell`
  (`parent.Spell`)
  (`Character.PlayAnimMontage` (`self.GetOwnerToCharacter`) "/Game/Character/Montages/MG_Fireball_03_Montage.MG_Fireball_03_Montage" 1.0 "None"))

(event `self.EndSpell`
  (`parent.EndSpell`))

(event `Throw`
  (bind _output_throwitemclass (break `/Game/Structs/FThrowItem` (`|GetArrayItem` (`self.ThrowItems`) (`self.CurrentItem`))))
  (`|SpawnActorFromClass` _output_throwitemclass (`KismetMathLibrary.MakeTransform` (`SceneComponent.GetSocketLocation` (`Character.Mesh` (`self.GetOwnerToCharacter`)) "Hand_Throw") (`Controller.GetControlRotation` (`GameplayStatics.GetPlayerController` 0)) (`self.ParticleScale`)) "Undefined" "OverrideRootScale" self null))

(fn `SetCurrentItem`
  (params (NewItem :type "/Game/Weapons/Magic/BP_ThrowItem Class Reference"))
  (locals (Index :type Integer))
  (bind (_output_throwitemclass _output_attachparticle) (break `/Game/Structs/FThrowItem` (`|GetArrayItem` (`self.ThrowItems`) (`self.CurrentItem`))))
  (bind _output_throwitemclass_2 (break `/Game/Structs/FThrowItem` (`|GetArrayItem` (`self.ThrowItems`) (`local.Index`))))
  (for (_ _array_index) (`self.ThrowItems`)
    (set `local.Index` _array_index)
    (if (== (`local.NewItem`) _output_throwitemclass_2)
      (break)))
  (set `self.CurrentItem` (`local.Index`))
  (`ParticleSystemComponent.SetTemplate` (`self.AttachParticle`) _output_attachparticle))

(fn `UserConstructionScript`
  (`parent.UserConstructionScript`))