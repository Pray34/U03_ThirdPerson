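; Player character that switches between unarmed, fist, sword and magic modes, with jumping or roll/backstep evades.
; Spawns weapon actors and HUD widgets at BeginPlay, forwards attacks to the current weapon, and cycles magic skills through a selection array.
; State gates equips and evades, while sphere-trace lock-on picks targets by dot product, switches by cross-product side and steers control rotation on Tick.
; Also handles aim zoom, a material-parameter radius effect and ragdoll-then-quit.
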(event `Key|X`
  (params (Key :type "Key Structure"))
  (:`Pressed`
    (`self.MakeRagdoll`)))

(event `MakeRagdoll`
  (bind _mesh (`self.Mesh`))
  (`PrimitiveComponent.SetCollisionEnabled` (`self.CapsuleComponent`) "NoCollision")
  (set `SpringArmComponent.bDoCollisionTest` false (`self.SpringArm`))
  (set `SkeletalMeshComponent.GlobalAnimRateScale` 0.0 (`self.Mesh`))
  (`PrimitiveComponent.SetSimulatePhysics` (`self.Mesh`) true)
  (`PrimitiveComponent.SetCollisionEnabled` _mesh "QueryAndPhysics")
  (`PrimitiveComponent.AddForce` _mesh (0.0 0.0 500000.0) "None" false)
  (`KismetSystemLibrary.Delay` 3.0)
  (`KismetSystemLibrary.ExecuteConsoleCommand` "Quit" (`GameplayStatics.GetPlayerController` 0)))

(event `self.ReceiveBeginPlay`
  (`|ExecutionSequence`
    (:`then_0`
      (bind _returnvalue (`|SpawnActorFromClass` "/Game/Weapons/Melee/BP_Sword.BP_Sword_C" (`KismetMathLibrary.MakeTransform` (0.0 0.0 0.0)) "Undefined" "OverrideRootScale" self null))
      (bind _output_get (set `self.Sword` _returnvalue))
      (`self.K2_AttachToComponent` _output_get (`self.Mesh`) "Holster_Sword" "KeepRelative" "KeepRelative" "KeepRelative" true))
    (:`then_1`
      (bind _returnvalue_2 (`|SpawnActorFromClass` "/Game/Weapons/Melee/BP_Fist.BP_Fist_C" (`KismetMathLibrary.MakeTransform` (0.0 0.0 0.0)) "Undefined" "OverrideRootScale" self null))
      (bind _output_get_2 (set `self.Fist` _returnvalue_2))
      (`self.K2_AttachToComponent` _output_get_2 (`self.Mesh`) "None" "KeepRelative" "KeepRelative" "KeepRelative" true))
    (:`then_2`
      (bind _returnvalue_3 (`|SpawnActorFromClass` "/Game/Weapons/Magic/BP_Magic.BP_Magic_C" (`KismetMathLibrary.MakeTransform` (0.0 0.0 0.0)) "Undefined" "OverrideRootScale" self null))
      (bind _output_get_3 (set `self.Magic` _returnvalue_3))
      (`self.K2_AttachToComponent` _output_get_3 (`self.Mesh`) "None" "KeepRelative" "KeepRelative" "KeepRelative" true))
    (:`then_3`
      (bind _returnvalue_4 (`|CreateWidget` "/Game/Widgets/WB_SkillContainer.WB_SkillContainer_C" (`GameplayStatics.GetPlayerController` 0)))
      (bind _output_get_4 (set `self.SkillWidget` _returnvalue_4))
      (`UserWidget.AddToViewport` _output_get_4 0)
      (`Widget.SetVisibility` (`self.SkillWidget`) "Hidden"))
    (:`then_4`
      (`|ExecutionSequence`
        (:`then_0`
          (`KismetArrayLibrary.Array_Add` (`self.SkillSelect`) (make `/Game/Structs/FSkillSelect` (`/Game/Weapons/Magic/BP_Magic.Heal` (`self.Magic`)))))
        (:`then_1`
          (`KismetArrayLibrary.Array_Add` (`self.SkillSelect`) (make `/Game/Structs/FSkillSelect` (`/Game/Weapons/Magic/BP_Magic.Warp` (`self.Magic`)))))
        (:`then_2`
          (`KismetArrayLibrary.Array_Add` (`self.SkillSelect`) (make `/Game/Structs/FSkillSelect` (`/Game/Weapons/Magic/BP_Magic.Throw` (`self.Magic`)) "/Game/Weapons/Magic/BP_FireBall.BP_FireBall_C")))
        (:`then_3`
          (`KismetArrayLibrary.Array_Add` (`self.SkillSelect`) (make `/Game/Structs/FSkillSelect` (`/Game/Weapons/Magic/BP_Magic.Throw` (`self.Magic`)) "/Game/Weapons/Magic/BP_ThunderBall.BP_ThunderBall_C")))))
    (:`then_5`
      (bind _returnvalue_5 (`|CreateWidget` "/Game/Widgets/WB_CrossHair.WB_CrossHair_C" (`GameplayStatics.GetPlayerController` 0)))
      (bind _output_get_5 (set `self.CrossHairWidget` _returnvalue_5))
      (`UserWidget.AddToViewport` _output_get_5 0)
      (`Widget.SetVisibility` _output_get_5 "Hidden"))))

(event `self.ReceiveTick`
  (params (DeltaSeconds :type "Float (single-precision)"))
  (`self.TickTargeting`))

(event `InputAxis|MoveForward`
  (params (AxisValue :type "Float (single-precision)"))
  (bind (_returnvalue_roll _returnvalue_pitch _returnvalue_yaw) (`KismetMathLibrary.BreakRotator` (`self.GetControlRotation`)))
  (if (`self.CanMove`)
    (`self.AddMovementInput` (`KismetMathLibrary.GetForwardVector` (`KismetMathLibrary.MakeRotator` 0.0 0.0 _returnvalue_yaw)) AxisValue)))

(event `InputAxis|MoveRight`
  (params (AxisValue :type "Float (single-precision)"))
  (bind (_returnvalue_roll _returnvalue_pitch _returnvalue_yaw) (`KismetMathLibrary.BreakRotator` (`self.GetControlRotation`)))
  (if (`self.CanMove`)
    (`self.AddMovementInput` (`KismetMathLibrary.GetRightVector` (`KismetMathLibrary.MakeRotator` 0.0 0.0 _returnvalue_yaw)) AxisValue)))

(event `InputAction|Walking`
  (params (Key :type "Key Structure"))
  (bind _charactermovement (`self.CharacterMovement`))
  (:`Pressed`
    (set `CharacterMovementComponent.MaxWalkSpeed` 400.0 _charactermovement))
  (:`Released`
    (set `CharacterMovementComponent.MaxWalkSpeed` 600.0 _charactermovement)))

(event `InputAction|Jumping`
  (params (Key :type "Key Structure"))
  (:`Pressed`
    (if (`self.CanMove`)
      (if (`|EnumEquality` (`self.CombatType`) "NewEnumerator0")
        (`self.Jump`)
        (else
          (`self.Evade`)))))
  (:`Released`
    (`self.StopJumping`)))

(event `Evade`
  (if (`|EnumEquality` (`self.StateType`) "NewEnumerator0")
    (if (< (`self.GetInputAxisValue`) 0.0)
      (set `self.StateType` "NewEnumerator5")
      (`self.PlayAnimMontage` "/Game/Character/Montages/BackStep_Montage.BackStep_Montage")
      (else
        (`|ExecutionSequence`
          (:`then_0`
            (set `self.bUseControllerRotationYaw` false)
            (set `CharacterMovementComponent.bOrientRotationToMovement` true (`self.CharacterMovement`)))
          (:`then_1`
            (`self.SetRollingDirection`)
            (set `self.StateType` "NewEnumerator6")
            (`self.PlayAnimMontage` "/Game/Character/Montages/Roll_Montage.Roll_Montage" 2.0)))))))

(event `BackStepped`
  (set `self.StateType` "NewEnumerator0"))

(event `Rolled`
  (set `self.StateType` "NewEnumerator0")
  (set `self.bUseControllerRotationYaw` true)
  (set `CharacterMovementComponent.bOrientRotationToMovement` false (`self.CharacterMovement`)))

(event `InputAxis|HorizontalLook`
  (params (AxisValue :type "Float (single-precision)"))
  (`self.AddControllerYawInput` AxisValue))

(event `InputAxis|VerticalLook`
  (params (AxisValue :type "Float (single-precision)"))
  (`self.AddControllerPitchInput` AxisValue))

(event `InputAction|Attack`
  (params (Key :type "Key Structure"))
  (:`Pressed`
    (bind _currentweapon (`self.CurrentWeapon`)
      (:`then`
        (`/Game/Weapons/BP_Weapon.Attack` _currentweapon))
      (:`else`))))

(event `InputAction|Targeting`
  (params (Key :type "Key Structure"))
  (:`Pressed`
    (`self.LockOnEnemy`
      (:`then`
        (`self.EndLockOn`))
      (:`else`
        (if (`|EnumInequality` (`self.CombatType`) "NewEnumerator0")
          (`self.StartLockOn`))))))

(event `StartLockOn`
  (`self.GetTraceTargets`)
  (`self.GetTargetEnemy`))

(event `EndLockOn`
  (bind _lockonenemy (`self.LockOnEnemy`)
    (:`then`
      (`SceneComponent.SetVisibility` (`/Game/Enemies/Enemy/BP_Enemy.TargetCursorWidget` _lockonenemy) false false)
      (set `self.LockOnEnemy` null)
      (`KismetArrayLibrary.Array_Clear` (`self.TracedEnemies`)))
    (:`else`)))

(event `TickTargeting`
  (`self.LockOnEnemy`
    (:`then`
      (if (> (`self.GetDistanceTo` (`self.LockOnEnemy`) self) (`self.LockOnDistance`))
        (`self.EndLockOn`)
        (else
          (`Controller.SetControlRotation` (`self.GetController`) (`KismetMathLibrary.FindLookAtRotation` (`self.K2_GetActorLocation`) (`self.K2_GetActorLocation` (`self.LockOnEnemy`)))))))
    (:`else`)))

(event `InputAction|TargetLeft`
  (params (Key :type "Key Structure"))
  (:`Pressed`
    (`self.GetNextTarget` false)))

(event `InputAction|TargetRight`
  (params (Key :type "Key Structure"))
  (:`Pressed`
    (`self.GetNextTarget` true)))

(event `InputAction|Fist`
  (params (Key :type "Key Structure"))
  (:`Pressed`
    (bind _result (`self.IsStateIdling`))
    (if _result
      (switch `/Game/Enums/ECombatType` (`self.CombatType`)
        (:`NewEnumerator0`
          (`self.EquipFist`))
        (:`NewEnumerator1`
          (bind _asbp_melee (cast `/Game/Weapons/Melee/BP_Melee` (`self.CurrentWeapon`)))
          (switch `/Game/Enums/EMeleeType` (`/Game/Weapons/Melee/BP_Melee.MeleeType` _asbp_melee)
            (:`NewEnumerator1`
              (`self.UnequipFist`))
            (:`NewEnumerator2`
              (`self.UnequipSword`)
              (set `self.ChangeFistMode` true))))
        (:`NewEnumerator2`
          (`self.UnequipMagic`)
          (`self.EquipFist`))))))

(event `EquipFist`
  (set `self.CombatType` "NewEnumerator1")
  (set `self.bUseControllerRotationYaw` true)
  (set `CharacterMovementComponent.bOrientRotationToMovement` false (`self.CharacterMovement`))
  (`self.SetCurrentWeapon` (`self.Fist`)))

(event `UnequipFist`
  (set `self.CanMove` true)
  (set `self.CombatType` "NewEnumerator0")
  (set `self.bUseControllerRotationYaw` false)
  (set `CharacterMovementComponent.bOrientRotationToMovement` true (`self.CharacterMovement`))
  (`self.SetCurrentWeapon` null))

(event `EquippedSword`
  (set `self.StateType` "NewEnumerator0")
  (set `self.CanMove` true)
  (set `self.CombatType` "NewEnumerator1")
  (set `self.bUseControllerRotationYaw` true)
  (set `CharacterMovementComponent.bOrientRotationToMovement` false (`self.CharacterMovement`))
  (`self.SetCurrentWeapon` (`self.Sword`)))

(event `EquipSword`
  (set `self.StateType` "NewEnumerator1")
  (`self.PlayAnimMontage` "/Game/Character/Montages/Draw_Sword_Montage.Draw_Sword_Montage" 0.8))

(event `UnequipSword`
  (set `self.StateType` "NewEnumerator2")
  (`self.PlayAnimMontage` "/Game/Character/Montages/Sheath_Sword_Montage.Sheath_Sword_Montage" 0.8))

(event `UnequippedSword`
  (set `self.StateType` "NewEnumerator0")
  (set `self.CanMove` true)
  (set `self.CombatType` "NewEnumerator0")
  (set `self.bUseControllerRotationYaw` false)
  (set `CharacterMovementComponent.bOrientRotationToMovement` true (`self.CharacterMovement`))
  (`self.SetCurrentWeapon` null)
  (`|ExecutionSequence`
    (:`then_0`
      (if (`self.ChangeFistMode`)
        (set `self.ChangeFistMode` false)
        (`self.EquipFist`)))
    (:`then_1`
      (if (`self.ChangeMagicMode`)
        (set `self.ChangeMagicMode` false)
        (`self.EquipMagic`)))))

(event `AttachSword`
  (`self.K2_AttachToComponent` (`self.Sword`) (`self.Mesh`) "Hand_Sword" "KeepRelative" "KeepRelative" "KeepRelative" true))

(event `DetachSword`
  (`self.K2_AttachToComponent` (`self.Sword`) (`self.Mesh`) "Holster_Sword" "KeepRelative" "KeepRelative" "KeepRelative" true))

(event `OnCollision`
  (`/Game/Weapons/Melee/BP_Sword.OnCollision` (`self.Sword`) "NewEnumerator0"))

(event `OffCollision`
  (`/Game/Weapons/Melee/BP_Sword.OffCollision` (`self.Sword`)))

(event `InputAction|Sword`
  (params (Key :type "Key Structure"))
  (:`Pressed`
    (bind _result (`self.IsStateIdling`))
    (if _result
      (switch `/Game/Enums/ECombatType` (`self.CombatType`)
        (:`NewEnumerator0`
          (`self.EquipSword`))
        (:`NewEnumerator1`
          (bind _asbp_melee (cast `/Game/Weapons/Melee/BP_Melee` (`self.CurrentWeapon`)))
          (switch `/Game/Enums/EMeleeType` (`/Game/Weapons/Melee/BP_Melee.MeleeType` _asbp_melee)
            (:`NewEnumerator1`
              (`self.UnequipFist`)
              (`self.EquipSword`))
            (:`NewEnumerator2`
              (`self.UnequipSword`))))
        (:`NewEnumerator2`
          (`self.UnequipMagic`)
          (`self.EquipSword`))))))

(event `EquipMagic`
  (set `self.CombatType` "NewEnumerator2")
  (set `self.bUseControllerRotationYaw` true)
  (set `CharacterMovementComponent.bOrientRotationToMovement` false (`self.CharacterMovement`))
  (`self.SetCurrentWeapon` (`self.Magic`))
  (`Widget.SetVisibility` (`self.SkillWidget`) "Visible")
  (`/Game/Widgets/WB_SkillContainer.OnMouseScroll` (`self.SkillWidget`) (`self.SkillIndex`)))

(event `UnequipMagic`
  (set `self.CanMove` true)
  (set `self.CombatType` "NewEnumerator0")
  (set `self.bUseControllerRotationYaw` false)
  (set `CharacterMovementComponent.bOrientRotationToMovement` true (`self.CharacterMovement`))
  (`self.SetCurrentWeapon` null)
  (`Widget.SetVisibility` (`self.SkillWidget`) "Hidden"))

(event `InputAction|Magic`
  (params (Key :type "Key Structure"))
  (:`Pressed`
    (bind _result (`self.IsStateIdling`))
    (if _result
      (switch `/Game/Enums/ECombatType` (`self.CombatType`)
        (:`NewEnumerator0`
          (`self.EquipMagic`))
        (:`NewEnumerator1`
          (bind _asbp_melee (cast `/Game/Weapons/Melee/BP_Melee` (`self.CurrentWeapon`)))
          (switch `/Game/Enums/EMeleeType` (`/Game/Weapons/Melee/BP_Melee.MeleeType` _asbp_melee)
            (:`NewEnumerator1`
              (`self.UnequipFist`)
              (`self.EquipMagic`))
            (:`NewEnumerator2`
              (`self.UnequipSword`)
              (set `self.ChangeMagicMode` true))))
        (:`NewEnumerator2`
          (`self.UnequipMagic`))))))

(event `OnAim`
  (`Widget.SetVisibility` (`self.CrossHairWidget`) "Visible")
  (bind (_direction _alpa) (`Timeline|타임라인_0` :!label _label)
    (:`Update`
      (set `SpringArmComponent.SocketOffset` (`KismetMathLibrary.VLerp` (0.0 0.0 0.0) (0.0 60.0 0.0) _alpa) (`self.SpringArm`))
      (`CameraComponent.SetFieldOfView` (`self.Camera`) (`KismetMathLibrary.Lerp` 90.0 45.0 _alpa)))))

(event `OffAim`
  (`Widget.SetVisibility` (`self.CrossHairWidget`) "Hidden")
  (goto _label :!via `Reverse`))

(event `InputAction|SkillLeft`
  (params (Key :type "Key Structure"))
  (bind _output_skill (break `/Game/Structs/FSkillSelect` (`|GetArrayItem` (`self.SkillSelect`) (`self.SkillIndex`))))
  (bind _output_skill_2 (break `/Game/Structs/FSkillSelect` (`|GetArrayItem` (`self.SkillSelect`) (`self.SkillIndex`))))
  (bind (_output_skill_3 _output_throwitemclass) (break `/Game/Structs/FSkillSelect` (`|GetArrayItem` (`self.SkillSelect`) (`self.SkillIndex`))))
  (:`Pressed`
    (switch `/Game/Enums/ECombatType` (`self.CombatType`)
      (:`NewEnumerator2`
        (bind _result (`/Engine/EditorBlueprintResources/StandardMacros.DecrementInt` (`self.SkillIndex`))
          (:`  `
            (if (< _result 0)
              (set `self.SkillIndex` (- (`KismetArrayLibrary.Array_Length` (`self.SkillSelect`)) 1)))
            (`/Game/Widgets/WB_SkillContainer.OnMouseScroll` (`self.SkillWidget`) (`self.SkillIndex`) :!label _label_2)
            (bind _asbp_skill_throw (cast `/Game/Weapons/Magic/BP_Skill_Throw` _output_skill_2)
              (:`then`
                (`/Game/Weapons/Magic/BP_Magic.SetCurrentSkill` (`self.Magic`) _output_skill_3)
                (`/Game/Weapons/Magic/BP_Skill_Throw.SetCurrentItem` _asbp_skill_throw _output_throwitemclass))
              (:`CastFailed`
                (`/Game/Weapons/Magic/BP_Magic.SetCurrentSkill` (`self.Magic`) _output_skill)))))))))

(event `InputAction|SkillRight`
  (params (Key :type "Key Structure"))
  (:`Pressed`
    (switch `/Game/Enums/ECombatType` (`self.CombatType`)
      (:`NewEnumerator2`
        (bind _result (`/Engine/EditorBlueprintResources/StandardMacros.IncrementInt` (`self.SkillIndex`))
          (:`  `
            (set `self.SkillIndex` (mod _result (`KismetArrayLibrary.Array_Length` (`self.SkillSelect`))))
            (goto _label_2)))))))

(event `Key|C`
  (params (Key :type "Key Structure"))
  (:`Pressed`
    (bind (_direction _out) (`Timeline|RadiousTimeline` :!via `PlayFromStart`)
      (:`Update`
        (`KismetMaterialLibrary.SetScalarParameterValue` "/Game/Materials/MPC_Radious.MPC_Radious" "Radious" _out)))))

(fn `GetComatType`
  (returns (OutCombatType :type "/Game/Enums/ECombatType Enum"))
  (return (`self.CombatType`)))

(fn `GetCurrentWeapon`
  (returns (CurrentWeapon :type "/Game/Weapons/BP_Weapon Object Reference"))
  (return (`self.CurrentWeapon`)))

(fn `GetNextTarget`
  (params (IsRight :type Boolean))
  (locals (EnemyElenemt :type "/Game/Enemies/Enemy/BP_Enemy Object Reference") (Map :type "Map of Float (double-precision) to /Game/Enemies/Enemy/BP_Enemy Object Reference") (Distance :type "Float (double-precision)") (Minimum :type "Float (double-precision)" :default 210000.0) (NextTarget :type "/Game/Enemies/Enemy/BP_Enemy Object Reference"))
  (bind _returnvalue (`KismetMathLibrary.Abs` (`local.Distance`)))
  (`self.LockOnEnemy`
    (:`then`
      (for _array_element (`self.TracedEnemies`)
        ;[1 1 1] 감지된 적의 거리를 맵에 등록
        (bind _output_get (set `local.EnemyElenemt` _array_element))
        (if (!= _output_get (`self.LockOnEnemy`))
          (bind _enemyelenemt (`local.EnemyElenemt`)
            (:`then`
              (`BlueprintMapLibrary.Map_Add` (`local.Map`) (`KismetMathLibrary.Dot_VectorVector` (`KismetMathLibrary.Cross_VectorVector` (`self.GetActorForwardVector`) (- (`self.K2_GetActorLocation` (`local.EnemyElenemt`)) (`self.K2_GetActorLocation`))) (`self.GetActorUpVector`)) _enemyelenemt))
            (:`else`))))
      ;[1 1 1] LockOnEnemy에 근접한 다음 타겟 찾기
      (bind _keys (`BlueprintMapLibrary.Map_Keys` (`local.Map`)))
      (for _array_element_2 _keys
        (set `local.Distance` _array_element_2)
        (if (`local.IsRight`)
          (if (>= (`local.Distance`) 0.0)
            (if (<= _returnvalue (`local.Minimum`)) :!label _label
              (set `local.Minimum` _returnvalue)
              (set `local.NextTarget` (`BlueprintMapLibrary.Map_Find` (`local.Map`) (`local.Distance`)))))
          (elif (< (`local.Distance`) 0.0)
            (goto _label))))
      (for _array_element_3 (`self.TracedEnemies`)
        (`/Engine/EditorBlueprintResources/StandardMacros.IsValid` _array_element_3
          (:`Is Valid`
            (`SceneComponent.SetVisibility` (`/Game/Enemies/Enemy/BP_Enemy.TargetCursorWidget` _array_element_3) false false)
            (bind _nexttarget (`local.NextTarget`)
              (:`then`
                (bind _output_get_2 (set `self.LockOnEnemy` _nexttarget))
                (`SceneComponent.SetVisibility` (`/Game/Enemies/Enemy/BP_Enemy.TargetCursorWidget` _output_get_2) true false))
              (:`else`
                (set `self.LockOnEnemy` null)))))))
    (:`else`)))

(fn `GetTargetEnemy`
  (locals (Maximum :type "Float (double-precision)") (FowardTarget :type "/Game/Enemies/Enemy/BP_Enemy Object Reference"))
  (for _array_element (`self.TracedEnemies`)
    (bind _returnvalue (`self.GetDotProductTo` _array_element))
    (if (>= _returnvalue (`local.Maximum`))
      (set `local.Maximum` _returnvalue)
      (set `local.FowardTarget` _array_element)))
  (bind _fowardtarget (`local.FowardTarget`)
    (:`then`
      (bind _output_get (set `self.LockOnEnemy` _fowardtarget))
      (`SceneComponent.SetVisibility` (`/Game/Enemies/Enemy/BP_Enemy.TargetCursorWidget` _output_get) true false))
    (:`else`
      (set `self.LockOnEnemy` null))))

(fn `GetTraceTargets`
  (bind _returnvalue (`self.K2_GetActorLocation`))
  (bind (_outhits _returnvalue_2) (`KismetSystemLibrary.SphereTraceMultiForObjects` _returnvalue (+ _returnvalue 1.0) (`self.LockOnDistance`) (`|MakeArray` "ObjectTypeQuery3" :!type "EObjectTypeQuery Enum")))
  (if _returnvalue_2
    (for _array_element _outhits
      (bind _asbp_enemy (cast `/Game/Enemies/Enemy/BP_Enemy` (`.HitActor` (`GameplayStatics.BreakHitResult` _array_element))))
      (`KismetArrayLibrary.Array_AddUnique` (`self.TracedEnemies`) _asbp_enemy))))

(fn `IsStateAttacking`
  (returns (Result :type Boolean))
  (return (`|EnumEquality` (`self.StateType`) "NewEnumerator3")))

(fn `IsStateIdling`
  (returns (Result :type Boolean))
  (return (`|EnumEquality` (`self.StateType`) "NewEnumerator0")))

(fn `SetCanMove`
  (params (InCanMove :type Boolean))
  (returns (Result :type Boolean))
  (set `self.CanMove` InCanMove)
  (return false))

(fn `SetCurrentWeapon`
  (params (NewWeapon :type "/Game/Weapons/BP_Weapon Object Reference"))
  (returns (Weapon :type "/Game/Weapons/BP_Weapon Object Reference"))
  (`/Engine/EditorBlueprintResources/StandardMacros.IsValid` (`self.CurrentWeapon`)
    (:`Is Valid`
      (`/Game/Weapons/BP_Weapon.OnUnequipped` (`self.CurrentWeapon`)))
    (:`Is Not Valid`
      _))
  (`/Engine/EditorBlueprintResources/StandardMacros.IsValid` (`local.NewWeapon`)
    (:`Is Valid`
      (bind _output_get (set `self.CurrentWeapon` (`local.NewWeapon`)))
      (`/Game/Weapons/BP_Weapon.OnEquipped` _output_get)
      (return _output_get))
    (:`Is Not Valid`
      (set `self.CurrentWeapon` null)
      (return null))))

(fn `SetRollingDirection`
  (bind _returnvalue (`self.K2_GetActorLocation`))
  (`self.K2_SetActorRotation` (`KismetMathLibrary.FindLookAtRotation` _returnvalue (+ _returnvalue (`KismetMathLibrary.Vector_Normal2D` (`self.GetVelocity`))))))

(fn `SetStateAttacking`
  (returns (Result :type Boolean))
  (set `self.StateType` "NewEnumerator3")
  (return false))

(fn `SetStateIdling`
  (returns (Result :type Boolean))
  (set `self.StateType` "NewEnumerator0")
  (return false))

(fn `SetStateSpelling`
  (returns (Result :type Boolean))
  (set `self.StateType` "NewEnumerator7")
  (return false))

(fn `UserConstructionScript`)